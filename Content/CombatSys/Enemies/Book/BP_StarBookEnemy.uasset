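; Stationary-looking star book enemy that turns to face the player and shoots little star projectiles.
; PawnSensing sightings trigger a yaw-only interpolated turn toward player 0, firing from ShootPoint after a short delay once yaw exactly matches.
; Incoming damage runs through BPDamageComponent, spawns a type-colored damage indicator, and destroys the actor at zero health.
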(event OnSeePawn(PawnSensing)
  (params (Pawn :type Pawn%20Object%20Reference))
  (Variables|Default|SetTarget Pawn)
  (Variables|Default|SetCanSeePlayer true)
  (CallFunction|FacePlayer))

(event Custom|FacePlayer
  (Variables|Default|SetCanAttack true)
  (if (Variables|Default|GetCanSeePlayer)
    (Transformation|SetActorRotation self (Math|Rotator|MakeRotator 0.0 0.0 (.yaw (Math|Interpolation|RInterpTo (Transformation|GetActorRotation) (Math|Rotator|FindLookatRotation (Transformation|GetActorLocation) (Transformation|GetActorLocation (Game|GetPlayerCharacter 0))) (* (Utilities|Time|GetWorldDeltaSeconds) 1e+02) 2e+01))))
    (if (== (.yaw (Transformation|GetActorRotation)) (.yaw (Math|Rotator|FindLookatRotation (Transformation|GetActorLocation) (Transformation|GetActorLocation (Game|GetPlayerCharacter 0)))))
      (if (Variables|Default|GetCanAttack)
        (Utilities|FlowControl|Delay 0.5)
        (CallFunction|Attack)
        (Utilities|FlowControl|Delay 1.0)))
    (else
      (Variables|Default|SetCanSeePlayer false))))

(event Custom|Attack
  (bind _shootpoint (Variables|Default|GetShootPoint))
  (Game|SpawnActorfromClass "/Game/CombatSys/SpellBP/Projectile_LittleStarV2.Projectile_LittleStarV2_C" (Math|Transform|MakeTransform (Transformation|GetWorldLocation _shootpoint) (Transformation|GetWorldRotation _shootpoint) "1.000000,1.000000,1.000000") "Undefined" "OverrideRootScale" 0 "NewEnumerator3" 0))

(event EventBeginPlay)

(event EventTick
  (params (DeltaSeconds :type Float%20%28single-precision%29)))

(event EventDie
  (params (KillingDamageType :type E_DamageTypes%20Enum :default "NewEnumerator0"))
  (Actor|DestroyActor))

(event EventTakeDamage
  (params (Damage :type Integer) (Damage%20Type :type E_DamageTypes%20Enum :default "NewEnumerator0") (DamageSource :type E_DamageSources%20Enum :default "NewEnumerator0"))
  (bind _bp_damagecomponent (Variables|Default|GetBP_DamageComponent))
  (bind _bp_damagecomponent_2 (Variables|Default|GetBP_DamageComponent))
  (bind _outgoingdamage (Default|CalculateDamage _bp_damagecomponent_2 Damage Damage%20Type DamageSource))
  (Game|SpawnActorfromClass "/Game/CombatSys/BP_DamageIndicator.BP_DamageIndicator_C" (Math|Transform|MakeTransform (+ (Transformation|GetWorldLocation (Variables|Character|GetMesh)) "0, 0,15.000000") "0, 0, 0" "1.000000,1.000000,1.000000") "Undefined" "OverrideRootScale" 0 (Utilities|Text|ToText(Integer) _outgoingdamage) (.Value (Utilities|Map|Find (Variables|/Game/ResourceSystem/BP_DamageComponent.BP_DamageComponent_C|GetDamageColours _bp_damagecomponent_2) Damage%20Type)) 0)
  (bind _output_get (Variables|/Game/ResourceSystem/BP_DamageComponent.BP_DamageComponent_C|SetCurrentHealth _bp_damagecomponent (- (Variables|/Game/ResourceSystem/BP_DamageComponent.BP_DamageComponent_C|GetCurrentHealth _bp_damagecomponent) _outgoingdamage)))
  (if (<= _output_get 0)
    (CallFunction|Die Damage%20Type)))

(event Collision|EventActorBeginOverlap
  (params (OtherActor :type Actor%20Object%20Reference)))

(fn ConstructionScript)