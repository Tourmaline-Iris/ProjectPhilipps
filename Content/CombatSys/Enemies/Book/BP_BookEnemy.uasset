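; BP_BookEnemy is a book enemy that chases the player and deals melee area damage.
; Pawn sensing triggers an AI move to player 0, then a delayed attack damages sphere-overlapping BPI_DamageDeath actors, excluding other books.
; Incoming damage goes through BPDamageComponent, spawns a coloured damage indicator, and destroys the book at zero health.
; The construction script randomly picks cover and binding materials using one shared index.
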(event OnSeePawn(PawnSensing)
  (params (Pawn :type Pawn%20Object%20Reference))
  (Variables|Default|SetTarget Pawn)
  (Variables|Default|SetCanSeePlayer true)
  (CallFunction|ChasePlayer))

(event Custom|ChasePlayer
  (Variables|Default|SetCanAttack true)
  (if (Variables|Default|GetCanSeePlayer)
    (AI|AIMoveTo self "0, 0, 0" (Game|GetPlayerCharacter 0) 5.0 true
      (:OnSuccess
        (if (Variables|Default|GetCanAttack)
          (Utilities|FlowControl|Delay 0.5)
          (CallFunction|Attack)
          (Utilities|FlowControl|Delay 1.0))))
    (else
      (Variables|Default|SetCanSeePlayer false))))

(event Custom|Attack
  (for _array_element (Collision|GetOverlappingActors (Variables|Default|GetSphere) 0 :!class /Script/Engine.PrimitiveComponent)
    (if (and (Utilities|DoesObjectImplementInterface _array_element "/Game/Blueprints/BPI_DamageDeath.BPI_DamageDeath_C") (!= (Utilities|GetClass _array_element) "BP_BookEnemy_C"))
      (Class|BPIDamageDeath|TakeDamage(Message) _array_element 10 "NewEnumerator0" "NewEnumerator1"))))

(event EventBeginPlay)

(event EventTick
  (params (DeltaSeconds :type Float%20%28single-precision%29)))

(event EventDie
  (params (KillingDamageType :type E_DamageTypes%20Enum :default "NewEnumerator0"))
  (Actor|DestroyActor))

(event EventTakeDamage
  (params (Damage :type Integer) (Damage%20Type :type E_DamageTypes%20Enum :default "NewEnumerator0") (DamageSource :type E_DamageSources%20Enum :default "NewEnumerator0"))
  (bind _bp_damagecomponent (Variables|Default|GetBP_DamageComponent))
  (bind _bp_damagecomponent_2 (Variables|Default|GetBP_DamageComponent))
  (bind _outgoingdamage (Default|CalculateDamage _bp_damagecomponent_2 Damage Damage%20Type DamageSource))
  (Game|SpawnActorfromClass "/Game/CombatSys/BP_DamageIndicator.BP_DamageIndicator_C" (Math|Transform|MakeTransform (+ (Transformation|GetWorldLocation (Variables|Character|GetMesh)) "0, 0,15.000000") "0, 0, 0" "1,1,1") "Undefined" 0 _outgoingdamage (.Value (Utilities|Map|Find (Variables|/Game/ResourceSystem/BP_DamageComponent.BP_DamageComponent_C|GetDamageColours _bp_damagecomponent_2) Damage%20Type)) 0)
  (bind _output_get (Variables|/Game/ResourceSystem/BP_DamageComponent.BP_DamageComponent_C|SetCurrentHealth _bp_damagecomponent (- (Variables|/Game/ResourceSystem/BP_DamageComponent.BP_DamageComponent_C|GetCurrentHealth _bp_damagecomponent) _outgoingdamage)))
  (if (<= _output_get 0)
    (CallFunction|Die Damage%20Type)))

(event Collision|EventActorBeginOverlap
  (params (OtherActor :type Actor%20Object%20Reference)))

(fn ConstructionScript
  (LocalVariables|SetL_Random (Math|Random|RandomIntegerinRange 0 (- (Utilities|Array|Length (Variables|Default|GetCoverColour)) 1)))
  (Rendering|Material|SetMaterial (Variables|Character|GetMesh) 0 (Utilities|Array|Get(acopy) (Variables|Default|GetCoverColour) (LocalVariables|GetL_Random)))
  (Rendering|Material|SetMaterial (Variables|Character|GetMesh) 2 (Utilities|Array|Get(acopy) (Variables|Default|GetBindingColour) (LocalVariables|GetL_Random))))