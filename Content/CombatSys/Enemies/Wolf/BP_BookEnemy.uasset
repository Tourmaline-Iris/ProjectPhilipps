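; BP_BookEnemy is a melee book enemy that chases the player on sight and damages what it reaches.
; PawnSensing starts an AI move to the player character, and a successful move triggers an attack after a short delay.
; The attack sends interface damage messages to BPI_DamageDeath actors overlapping its sphere.
; The construction script randomises the book's look, using one index for both cover and binding materials.
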(event OnSeePawn(PawnSensing)
  (params (Pawn :type Pawn%20Object%20Reference))
  (Variables|Default|SetTarget Pawn)
  (Variables|Default|SetCanSeePlayer true)
  (CallFunction|ChasePlayer))

(event Custom|ChasePlayer
  (Variables|Default|SetCanAttack true)
  (if (Variables|Default|GetCanSeePlayer)
    (AI|AIMoveTo self "0, 0, 0" (Game|GetPlayerCharacter 0) 5.0 true
      (:OnSuccess
        (if (Variables|Default|GetCanAttack)
          (Utilities|FlowControl|Delay 0.5)
          (CallFunction|Attack)
          (Utilities|FlowControl|Delay 1.0))))
    (else
      (Variables|Default|SetCanSeePlayer false))))

(event Custom|Attack
  (for _array_element (Collision|GetOverlappingActors (Variables|Default|GetSphere) 0 :!class /Script/Engine.PrimitiveComponent)
    (if (Utilities|DoesObjectImplementInterface _array_element "/Game/Blueprints/BPI_DamageDeath.BPI_DamageDeath_C")
      (Class|BPIDamageDeath|TakeDamage(Message) _array_element 10 "NewEnumerator0" "NewEnumerator1"))))

(event EventBeginPlay)

(event Collision|EventActorBeginOverlap
  (params (OtherActor :type Actor%20Object%20Reference)))

(event EventTick
  (params (DeltaSeconds :type Float%20%28single-precision%29)))

(fn ConstructionScript
  (LocalVariables|SetL_Random (Math|Random|RandomIntegerinRange 0 (- (Utilities|Array|Length (Variables|Default|GetCoverColour)) 1)))
  (Rendering|Material|SetMaterial (Variables|Character|GetMesh) 0 (Utilities|Array|Get(acopy) (Variables|Default|GetCoverColour) (LocalVariables|GetL_Random)))
  (Rendering|Material|SetMaterial (Variables|Character|GetMesh) 2 (Utilities|Array|Get(acopy) (Variables|Default|GetBindingColour) (LocalVariables|GetL_Random))))