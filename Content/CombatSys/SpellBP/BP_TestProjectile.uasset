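; BP_TestProjectile is a test spell projectile that damages what it overlaps and destroys itself.
; On overlap it prints a debug string, then skips actors that share its owner.
; Other actors implementing BPI_DamageDeath receive a TakeDamageMessage with its damage and type, after which the projectile is destroyed.
; Any hit event also destroys it.
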(event EventBeginPlay
  (|CallParentFunction) ; This node is disabled and will not be called.\nDrag off pins to build functionality.
)

(event Collision|EventActorBeginOverlap
  (params (OtherActor :type Actor%20Object%20Reference))
  (Development|PrintString "Overlap")
  (if (not (== (Components|GetOwner OtherActor) (Components|GetOwner)))
    (Utilities|Casting|CastToBPI_DamageDeath OtherActor)
    (Class|BPIDamageDeath|TakeDamage(Message) OtherActor (Variables|Default|GetDamage) (Variables|Default|GetDamageType) "NewEnumerator0")
    (Actor|DestroyActor)))

(event Collision|EventHit
  (params (MyComp :type Primitive%20Component%20Object%20Reference) (Other :type Actor%20Object%20Reference) (OtherComp :type Primitive%20Component%20Object%20Reference) (bSelfMoved :type Boolean) (HitLocation :type Vector :default "0, 0, 0") (HitNormal :type Vector :default "0, 0, 0") (NormalImpulse :type Vector :default "0, 0, 0") (Hit :type Hit%20Result%20Structure%20%28by%20ref%29))
  (Actor|DestroyActor))

(fn ConstructionScript
  (|CallParentFunction))