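; BP_PolarisShield is a temporary, damageable shield actor from the combat system's spell Blueprints.
; On BeginPlay it fills its damage component's health, copies its team onto that component, and destroys itself after a set duration.
; Incoming damage passes through the component's CalculateDamage before reducing health, and the shield is destroyed early once health reaches zero.
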(event EventBeginPlay
  (bind _bp_damagecomponent (Variables|Default|GetBP_DamageComponent))
  (Variables|/Game/ResourceSystem/BP_DamageComponent.BP_DamageComponent_C|SetCurrentHealth _bp_damagecomponent (Variables|/Game/ResourceSystem/BP_DamageComponent.BP_DamageComponent_C|GetMaxHealth _bp_damagecomponent))
  (Variables|/Game/ResourceSystem/BP_DamageComponent.BP_DamageComponent_C|SetTeam _bp_damagecomponent (Variables|Default|GetObjectTeam))
  (Utilities|FlowControl|Delay (Variables|Default|GetDuration))
  (Actor|DestroyActor))

(event EventTakeDamage
  (params (Damage :type Integer) (Damage%20Type :type E_DamageTypes%20Enum :default "NewEnumerator0") (DamageSource :type E_DamageSources%20Enum :default "NewEnumerator0"))
  (bind _bp_damagecomponent (Variables|Default|GetBP_DamageComponent))
  (bind _output_get (Variables|/Game/ResourceSystem/BP_DamageComponent.BP_DamageComponent_C|SetCurrentHealth _bp_damagecomponent (- (Variables|/Game/ResourceSystem/BP_DamageComponent.BP_DamageComponent_C|GetCurrentHealth _bp_damagecomponent) (.OutgoingDamage (Default|CalculateDamage (Variables|Default|GetBP_DamageComponent) Damage Damage%20Type DamageSource)))))
  (if (<= _output_get 0)
    (CallFunction|Die Damage%20Type)))

(event EventDie
  (params (KillingDamageType :type E_DamageTypes%20Enum :default "NewEnumerator0"))
  (Actor|DestroyActor))

(fn ConstructionScript)