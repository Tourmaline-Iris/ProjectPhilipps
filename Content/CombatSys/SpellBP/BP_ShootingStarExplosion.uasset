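; BP_ShootingStarExplosion is the short-lived explosion actor for the Shooting Star spell, damaging actors it overlaps.
; Tick lerps its scale from StartScale to EndScale over Lifetime, while BeginPlay destroys it after a fixed delay independent of that variable.
; On overlap, it sends TakeDamageMessage through BPI_DamageDeath to actors whose BP_DamageComponent team differs from its ObjectTeam, with a leftover debug print.
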(event Collision|EventActorBeginOverlap
  (params (OtherActor :type Actor%20Object%20Reference))
  (bind _output_get (Variables|Default|SetHItActor OtherActor))
  (bind _output_get_2 (Variables|Default|SetHitActorDamageComp (Actor|GetComponentbyClass _output_get "/Game/ResourceSystem/BP_DamageComponent.BP_DamageComponent_C")))
  (if (Utilities|IsValid (Actor|GetComponentbyClass _output_get "/Game/ResourceSystem/BP_DamageComponent.BP_DamageComponent_C"))
    (if (not (Utilities|Enum|Equal(Enum) (Variables|/Game/ResourceSystem/BP_DamageComponent.BP_DamageComponent_C|GetTeam _output_get_2) (Variables|Default|GetObjectTeam)))
      (if (Utilities|DoesObjectImplementInterface (Variables|Default|GetHItActor) "/Game/Blueprints/BPI_DamageDeath.BPI_DamageDeath_C")
        (Development|PrintString "Trying to deal damage")
        (Class|BPIDamageDeath|TakeDamage(Message) (Variables|Default|GetHitActor) (Variables|Default|GetDamage) (Variables|Default|GetDamageType) "NewEnumerator0")))))

(event EventBeginPlay
  (Utilities|FlowControl|Delay 0.2)
  (Actor|DestroyActor))

(event EventTick
  (params (DeltaSeconds :type Float%20%28single-precision%29))
  (Transformation|SetActorRelativeScale3D (Math|Conversions|ToVector(Float) (Math|Float|Lerp (Variables|Default|GetStartScale) (Variables|Default|GetEndScale) (/ (Actor|GetGameTimeSinceCreation) (Variables|Default|GetLifetime))))))

(fn ConstructionScript)