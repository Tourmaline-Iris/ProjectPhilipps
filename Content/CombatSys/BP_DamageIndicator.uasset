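; BP_DamageIndicator is an actor that shows a floating damage number in the world.
; On BeginPlay it passes its damage amount and colour to a WBP_FloatingDamage widget held in its widget component.
; A random upward and sideways impulse on its static mesh tosses the indicator into the air, and the actor destroys itself after a short delay.
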(event EventBeginPlay
  (bind _aswbp_floating_damage (Utilities|Casting|CastToWBP_FloatingDamage (UserInterface|GetUserWidgetObject (Variables|Default|GetWidget))))
  (Default|SetText _aswbp_floating_damage (Variables|Default|GetDamage) (Variables|Default|GetDamageColour))
  (Physics|AddImpulse (Variables|Default|GetStaticMesh) (Math|Vector|MakeVector (Math|Random|RandomFloatinRange -4e+02 4e+02) (Math|Random|RandomFloatinRange -4e+02 4e+02) (Math|Random|RandomFloatinRange 4e+02 8e+02)) "None" false)
  (Utilities|FlowControl|Delay 2.0)
  (Actor|DestroyActor))

(fn ConstructionScript)