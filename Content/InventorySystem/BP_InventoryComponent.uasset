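; Inventory component that stores a fixed number of item slots as structs of item class, quantity and typed subdata maps.
; BeginPlay sizes the contents and slot-reference arrays, then runs each entry through AddMissingSubdata.
; That function copies any bool, int, float or string keys the item lacks from its class defaults, keeping existing values.
; Setting an item by index applies the same fill and refreshes the matching slot.
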(event EventBeginPlay
  (Utilities|Array|Resize (Variables|Default|GetContents) (Variables|Default|GetSlotNumber))
  (Utilities|Array|Resize (Variables|Default|GetSlotref) (Variables|Default|GetSlotNumber))
  (for (_array_element _array_index) (Variables|Default|GetContents)
    (bind _itemoutput (CallFunction|AddMissingSubdata _array_element))
    (Utilities|Array|SetArrayElem (Variables|Default|GetContents) _array_index _itemoutput)))

(fn SetItemInfoatIndex
  (params (Index :type Integer) (Item :type Inventory%20Content%20Struct%20Structure))
  (bind _itemoutput (CallFunction|AddMissingSubdata Item))
  (bind _output_get (LocalVariables|SetL_Index Index))
  (Utilities|Array|SetArrayElem (Variables|Default|GetContents) _output_get _itemoutput true)
  (Default|UpdateSlot (Utilities|Array|Get(acopy) (Variables|Default|GetSlotref) (LocalVariables|GetL_Index)))
  (return))

(fn GetItemInfoatIndex
  (params (Index :type Integer))
  (LocalVariables|SetL_Index Index)
  (return (Utilities|Array|Get(acopy) (Variables|Default|GetContents) (LocalVariables|GetL_Index))))

(fn ValidateItemSlot
  (params (Index :type Integer))
  (LocalVariables|SetL_Index Index)
  (return (Utilities|IsValidClass (.itemtype (Utilities|Array|Get(acopy) (Variables|Default|GetContents) (LocalVariables|GetL_Index))))))

(fn AddMissingSubdata
  (params (ItemInput :type Inventory%20Content%20Struct%20Structure))
  (bind _subdata (Utilities|GetClassDefaults (.itemtype ItemInput)))
  (if (Utilities|IsValidClass (.itemtype ItemInput))
    (LocalVariables|SetL_SubdataStr (.subdata_str (.subdata ItemInput)))
    (LocalVariables|SetL_SubdataBool (.subdata_bool (.subdata ItemInput)))
    (LocalVariables|SetL_SubdataInt (.subdata_int (.subdata ItemInput)))
    (LocalVariables|SetL_SubdataFloat (.subdata_float (.subdata ItemInput)))
    (Utilities|FlowControl|Sequence
      (:then_0
        (bind _keys (Utilities|Map|Keys (.subdata_bool _subdata)))
        (for _array_element _keys
          (if (not (.ReturnValue (Utilities|Map|Find (LocalVariables|GetL_SubdataBool) _array_element)))
            (Utilities|Map|Add (LocalVariables|GetL_SubdataBool) _array_element (.Value (Utilities|Map|Find (.subdata_bool _subdata) _array_element))))))
      (:then_1
        (bind _keys_2 (Utilities|Map|Keys (.subdata_int _subdata)))
        (for _array_element_2 _keys_2
          (if (not (.ReturnValue (Utilities|Map|Find (LocalVariables|GetL_SubdataInt) _array_element_2)))
            (Utilities|Map|Add (LocalVariables|GetL_SubdataInt) _array_element_2 (.Value (Utilities|Map|Find (.subdata_int _subdata) _array_element_2))))))
      (:then_2
        (bind _keys_3 (Utilities|Map|Keys (.subdata_float _subdata)))
        (for _array_element_3 _keys_3
          (if (not (.ReturnValue (Utilities|Map|Find (LocalVariables|GetL_SubdataFloat) _array_element_3)))
            (Utilities|Map|Add (LocalVariables|GetL_SubdataFloat) _array_element_3 (.Value (Utilities|Map|Find (.subdata_float _subdata) _array_element_3))))))
      (:then_3
        (bind _keys_4 (Utilities|Map|Keys (.subdata_str _subdata)))
        (for _array_element_4 _keys_4
          (if (not (.ReturnValue (Utilities|Map|Find (LocalVariables|GetL_SubdataStr) _array_element_4)))
            (Utilities|Map|Add (LocalVariables|GetL_SubdataStr) _array_element_4 (.Value (Utilities|Map|Find (.subdata_str _subdata) _array_element_4))))))
      (:then_4
        (return (Utilities|Struct|MakeInventoryContentStruct (.itemtype ItemInput) (.quantity ItemInput) (Utilities|Struct|MakeItemSubdataStruct (LocalVariables|GetL_SubdataBool) (LocalVariables|GetL_SubdataInt) (LocalVariables|GetL_SubdataFloat) (LocalVariables|GetL_SubdataStr))))))
    (else
      (return ""))))