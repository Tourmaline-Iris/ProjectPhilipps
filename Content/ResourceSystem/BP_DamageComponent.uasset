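; Damage component that resolves a hit into a final integer amount and display text, based on damage type and damage source.
; CalculateDamage zeroes the hit on either immunity, otherwise truncates damage times both map-based multipliers.
; Map lookups ignore the found flag, so a missing multiplier entry yields zero damage.
; FormatText shows "[X]" for immunity or the number, adding "!" when either multiplier exceeds one.
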(fn CalculateDamage
  (params (Damage :type Integer) (DamageType :type E_DamageTypes%20Enum :default "NewEnumerator0") (DamageSource :type E_DamageSources%20Enum :default "NewEnumerator0"))
  (bind _damagetypemults (Variables|Default|GetDamageTypeMults))
  (bind _damagesourcemults (Variables|Default|GetDamageSourceMults))
  (bind _damagetypeimmunities (Variables|Default|GetDamageTypeImmunities))
  (bind _damagesourceimmunities (Variables|Default|GetDamageSourceImmunities))
  (bind _value (Utilities|Map|Find _damagesourcemults DamageSource))
  (bind _value_2 (Utilities|Map|Find _damagetypemults DamageType))
  (bind _value_3 (Utilities|Map|Find _damagetypeimmunities DamageType))
  (bind _value_4 (Utilities|Map|Find _damagesourceimmunities DamageSource))
  (bind _returnvalue (* _value_2 _value))
  (bind _returnvalue_2 (or _value_3 _value_4))
  (bind _returnvalue_3 (* Damage _returnvalue))
  (bind _returnvalue_4 (Math|Float|Truncate _returnvalue_3))
  (bind _returnvalue_5 (select _returnvalue_2 0 _returnvalue_4))
  (bind _damagetext (CallFunction|FormatText _returnvalue_5 _returnvalue_2 (or (> _value_2 1.0) (> _value 1.0))))
  (return _returnvalue_5 _damagetext))

(fn FormatText
  (params (Damage :type Integer) (IsImmune :type Boolean) (IsAmplified :type Boolean))
  (bind _returnvalue (Utilities|Text|ToText(Integer) Damage))
  (bind _returnvalue_2 (select IsImmune "[X]" _returnvalue))
  (return (select IsAmplified (Utilities|Text|FormatText "{text}!" _returnvalue_2) _returnvalue_2)))