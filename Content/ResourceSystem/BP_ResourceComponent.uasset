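; BP_ResourceComponent drops loot for its owning BP_MasterResource from a weighted loot table.
; DropLoot sums the table's weights, rolls a random number up to that total, and walks the entries, subtracting weights until one is selected.
; It spawns that single item at the owner's DropLocation and applies an upward impulse with random horizontal strength to its static mesh.
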(fn DropLoot
  (params (LootTable :type Map%20of%20BP%20Master%20Item%20Class%20References%20to%20Reals))
  (LocalVariables|SetL_Sum 0.0)
  (LocalVariables|SetL_RandomNumber 0.0)
  (LocalVariables|SetL_LootTable LootTable)
  (Utilities|FlowControl|Sequence
    (:then_0
      (bind _values (Utilities|Map|Values (LocalVariables|GetL_LootTable)))
      (for _array_element _values
        (LocalVariables|SetL_Sum (+ _array_element (LocalVariables|GetL_Sum)))))
    (:then_1
      (LocalVariables|SetL_RandomNumber (Math|Random|RandomFloatinRange 0.0 (LocalVariables|GetL_Sum)))
      (bind _keys (Utilities|Map|Keys (LocalVariables|GetL_LootTable)))
      (for _array_element_2 _keys
        (if (< (LocalVariables|GetL_RandomNumber) (.Value (Utilities|Map|Find (LocalVariables|GetL_LootTable) _array_element_2)))
          (bind _returnvalue (Game|SpawnActorfromClass :Class _array_element_2 :SpawnTransform (Math|Transform|MakeTransform (Transformation|GetWorldLocation (Variables|/Game/ResourceSystem/BP_MasterResource.BP_MasterResource_C|GetDropLocation (.AsBP%20Master%20Resource (Utilities|Casting|CastToBP_MasterResource (Components|GetOwner))))) "0, 0, 0" "1.000000,1.000000,1.000000") :CollisionHandlingOverride "AdjustIfPossibleButAlwaysSpawn" :TransformScaleMethod "SelectDefaultAtRuntime" :Instigator 0))
          (Physics|AddImpulse (Variables|/Game/ItemSystem/BP_MasterItem.BP_MasterItem_C|GetStaticMesh _returnvalue) (Math|Vector|MakeVector (Math|Random|RandomFloatinRange 0.0 (LocalVariables|GetImpulseStrength)) (Math|Random|RandomFloatinRange 0.0 (LocalVariables|GetImpulseStrength)) 2e+02) "None" false)
          (return)
          (else
            (LocalVariables|SetL_RandomNumber (- (LocalVariables|GetL_RandomNumber) (.Value (Utilities|Map|Find (LocalVariables|GetL_LootTable) _array_element_2))))))))))