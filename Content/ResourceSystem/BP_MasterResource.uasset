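; Base actor for damageable resources that drop loot when destroyed.
; BPDamageComponent holds team and health and calculates incoming damage, which TakeDamage shows through a spawned, type-coloured damage indicator and subtracts from health.
; At zero health, Die picks the loot table and drop count matching the killing damage type from SpecialLootTables, falling back to defaults.
; BPResourceComponent then drops the loot before the actor destroys itself.
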(event EventDie
  (params (KillingDamageType :type E_DamageTypes%20Enum :default "NewEnumerator0"))
  (bind (_table _drop_number) (CallFunction|SetLootTable KillingDamageType))
  (for _index (range 1 _drop_number)
    (Default|DropLoot (Variables|Default|GetBP_ResourceComponent) _table))
  (Actor|DestroyActor))

(event EventTakeDamage
  (params (Damage :type Integer) (Damage%20Type :type E_DamageTypes%20Enum :default "NewEnumerator0") (DamageSource :type E_DamageSources%20Enum :default "NewEnumerator0"))
  (bind _bp_damagecomponent (Variables|Default|GetBP_DamageComponent))
  (bind _bp_damagecomponent_2 (Variables|Default|GetBP_DamageComponent))
  (bind (_outgoingdamage _damagetext) (Default|CalculateDamage _bp_damagecomponent_2 Damage Damage%20Type DamageSource))
  (Game|SpawnActorfromClass "/Game/CombatSys/BP_DamageIndicator.BP_DamageIndicator_C" (Math|Transform|MakeTransform (+ (Transformation|GetWorldLocation (Variables|Default|GetStaticMesh)) "0, 0,15.000000") "0, 0, 0" "1.000000,1.000000,1.000000") "Undefined" "OverrideRootScale" 0 _damagetext (.Value (Utilities|Map|Find (Variables|/Game/ResourceSystem/BP_DamageComponent.BP_DamageComponent_C|GetDamageColours (Variables|Default|GetBP_DamageComponent)) Damage%20Type)) 0)
  (bind _output_get (Variables|/Game/ResourceSystem/BP_DamageComponent.BP_DamageComponent_C|SetCurrentHealth _bp_damagecomponent (- (Variables|/Game/ResourceSystem/BP_DamageComponent.BP_DamageComponent_C|GetCurrentHealth _bp_damagecomponent) _outgoingdamage)))
  (if (<= _output_get 0)
    (CallFunction|Die Damage%20Type)))

(event EventBeginPlay
  (bind _bp_damagecomponent (Variables|Default|GetBP_DamageComponent))
  (Variables|/Game/ResourceSystem/BP_DamageComponent.BP_DamageComponent_C|SetTeam _bp_damagecomponent (Variables|Damage|GetObjectTeam))
  (Variables|/Game/ResourceSystem/BP_DamageComponent.BP_DamageComponent_C|SetCurrentHealth _bp_damagecomponent (Variables|/Game/ResourceSystem/BP_DamageComponent.BP_DamageComponent_C|GetMaxHealth _bp_damagecomponent)))

(fn ConstructionScript)

(fn SetLootTable
  (params (DamageType :type E_DamageTypes%20Enum :default "NewEnumerator0"))
  (for _array_element (Variables|CustomLootTables|GetSpecialLootTables)
    (if (Utilities|Enum|Equal(Enum) (.damagetype _array_element) DamageType)
      (return (.loottable _array_element) (.numberofdrops _array_element))))
  (return (Variables|LootTables|GetDefaultLootTable) (Variables|LootTables|GetDefaultDropNum)))