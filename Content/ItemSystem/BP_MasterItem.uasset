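; Master item actor for world pickups that move into the player's inventory on interaction.
; Interact measures matching inventory space, adds what fits and pushes an indicator widget to the HUD.
; Unless space exceeds the stack, it spawns a same-class actor holding the remainder, then destroys itself whenever any space was found.
; The construction script validates the item's Subdata, which is also used to match inventory stacks.
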(event EventInteract
  (params (PlayerRef :type First%20Person%20Character%20Object%20Reference))
  (bind _self self)
  (bind _self_2 self)
  (bind _self_3 self)
  (bind _output_get (Variables|Default|SetPlayerRef PlayerRef))
  (bind _runningtotal (CallFunction|FindSpaceonPlayer _output_get (Utilities|Struct|MakeInventoryContentStruct (Utilities|GetClass self) (Variables|Default|GetItemQuantity) (Variables|Default|GetSubdata)) true))
  (if (> _runningtotal 0)
    (if (> _runningtotal (Variables|Default|GetItemQuantity))
      (CallFunction|AddItemtoInventory (Variables|Default|GetPlayerRef) (Utilities|Struct|MakeInventoryContentStruct (Utilities|GetClass _self_2) (Variables|Default|GetItemQuantity) (Variables|Default|GetSubdata _self_2)))
      (bind _returnvalue (Game|ConstructObjectfromClass self "/Game/InventorySystem/UI/WBP_AddItemIndicator.WBP_AddItemIndicator_C" (Variables|Default|GetItemQuantity) (Utilities|GetClass self)))
      (Class|Widget|SetRenderTransformAngle _returnvalue 1.8e+02)
      (Class|VerticalBox|AddChildtoVerticalBox (Variables|/Game/Blueprints/HUD/WBP_HUD.WBP_HUD_C|GetAddItemBox (Variables|/Game/FirstPersonBP/Blueprints/FirstPersonCharacter.FirstPersonCharacter_C|GetHudRef (Variables|Default|GetPlayerRef))) _returnvalue)
      (Actor|DestroyActor)
      (else
        (CallFunction|AddItemtoInventory (Variables|Default|GetPlayerRef) (Utilities|Struct|MakeInventoryContentStruct (Utilities|GetClass _self) _runningtotal (Variables|Default|GetSubdata _self)))
        (Game|SpawnActorfromClass (Utilities|GetClass _self_3) (Math|Transform|MakeTransform (Transformation|GetWorldLocation (Variables|Default|GetSphere)) "0, 0, 0" "1.000000,1.000000,1.000000") "AlwaysSpawn" "SelectDefaultAtRuntime" 0 (- (Variables|Default|GetItemQuantity) _runningtotal) (Variables|Default|GetSubdata _self_3) 0)
        (bind _returnvalue_2 (Game|ConstructObjectfromClass self "/Game/InventorySystem/UI/WBP_AddItemIndicator.WBP_AddItemIndicator_C" (- (Variables|Default|GetItemQuantity) _runningtotal) (Utilities|GetClass self)))
        (Class|Widget|SetRenderTransformAngle _returnvalue_2 1.8e+02)
        (Class|VerticalBox|AddChildtoVerticalBox (Variables|/Game/Blueprints/HUD/WBP_HUD.WBP_HUD_C|GetAddItemBox (Variables|/Game/FirstPersonBP/Blueprints/FirstPersonCharacter.FirstPersonCharacter_C|GetHudRef (Variables|Default|GetPlayerRef))) _returnvalue_2)
        (Actor|DestroyActor)))))

(fn ConstructionScript
  (bind _itemoutput (CallFunction|ValidateSubdata (Utilities|Struct|MakeInventoryContentStruct (Utilities|GetClass self) (Variables|Default|GetItemQuantity) (Variables|Default|GetSubdata))))
  (Variables|Default|SetSubdata (.subdata _itemoutput))
  (if true
    _))