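; Resource component that gives its owning actor damageable health and drops loot on death, though BeginPlay currently calls Die immediately.
; TakeDamage scales damage by a per-type multiplier map and calls Die at zero health, which runs DropLoot and destroys the owner.
; DropLoot makes a weighted roll over the Resources class-to-weight map, spawning above the owner.
; The roll loop never breaks, so several items can spawn.
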(event EventBeginPlay
  (CallFunction|Die "NewEnumerator0"))

(event EventTakeDamage
  (params (Damage :type Integer) (Damage%20Type :type E_DamageTypes%20Enum :default "NewEnumerator0"))
  (bind _outgoingdamage (CallFunction|CalculateDamage Damage Damage%20Type))
  (bind _output_get (Variables|Default|SetCurrentHealth (- (Variables|Default|GetCurrentHealth) _outgoingdamage)))
  (if (<= _output_get 0)
    (CallFunction|Die Damage%20Type)))

(event EventDie
  (params (KillingDamageType :type E_DamageTypes%20Enum :default "NewEnumerator0"))
  (CallFunction|DropLoot KillingDamageType)
  (Actor|DestroyActor (Components|GetOwner)))

(fn CalculateDamage
  (params (Damage :type Integer) (DamageType :type E_DamageTypes%20Enum :default "NewEnumerator0"))
  (return (Math|Float|Truncate (* Damage (.Value (Utilities|Map|Find (Variables|Default|GetDamageMults) DamageType))))))

(fn DropLoot
  (params (Damage%20Type :type E_DamageTypes%20Enum :default "NewEnumerator0"))
  (Utilities|FlowControl|Sequence
    (:then_0
      (bind _values (Utilities|Map|Values (Variables|Default|GetResources)))
      (for _array_element _values
        (LocalVariables|SetL_Sum (+ _array_element (LocalVariables|GetL_Sum)))))
    (:then_1
      (LocalVariables|SetL_RandomNumber (Math|Random|RandomFloatinRange 0.0 (LocalVariables|GetL_Sum)))
      (bind _keys (Utilities|Map|Keys (Variables|Default|GetResources)))
      (for _array_element_2 _keys
        (if (< (LocalVariables|GetL_RandomNumber) (.Value (Utilities|Map|Find (Variables|Default|GetResources) _array_element_2)))
          (Game|SpawnActorfromClass :Class _array_element_2 :SpawnTransform (Math|Transform|MakeTransform (+ (Transformation|GetActorLocation (Components|GetOwner)) "0, 0,100.000000") "0, 0, 0" "1,1,1") :CollisionHandlingOverride "AlwaysSpawn" :Instigator 0)
          (else
            (LocalVariables|SetL_RandomNumber (- (LocalVariables|GetL_RandomNumber) (.Value (Utilities|Map|Find (Variables|Default|GetResources) _array_element_2))))))))))