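; Blueprint function library for BPAS, a tag-driven ability system built on ability, attribute and gameplay tag manager components.
; An actor counts as having BPAS if it has the ability manager, and a shared lookup then returns all three components.
; That lookup feeds tag checks and ability event broadcasts.
; Ability definitions are found by scanning a data table for an exact tag match; Edit Attribute is an empty stub.
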(fn BPASGetAbilityTagbyDefinition
  (params (Ability%20Tag :type Gameplay%20Tag%20Structure))
  (bind _outrownames (DataTable|GetDataTableRowNames "/Game/BPAS/Data/DataTables/TBL_AbilityDefinitions.TBL_AbilityDefinitions"))
  (bind _array_element (Utilities|Array|ForEachLoopwithBreak _outrownames :!label _label)
    (:LoopBody
      (bind _returnvalue (Utilities|GetDataTableRow "/Game/BPAS/Data/DataTables/TBL_AbilityDefinitions.TBL_AbilityDefinitions" _array_element)
        (:then
          (if (GameplayTags|MatchesTag (.AbilityTag (Utilities|Struct|BreakStruct_AbilityBaseData _returnvalue)) Ability%20Tag true)
            (LocalVariables|SetL_FoundAbilityDefinition? (GameplayTags|MatchesTag (.AbilityTag (Utilities|Struct|BreakStruct_AbilityBaseData _returnvalue)) Ability%20Tag true))
            (LocalVariables|SetL_AbilityDefinitionFound _returnvalue)
            (goto _label Break)))))
    (:Completed
      (return (LocalVariables|GetL_FoundAbilityDefinition?) (LocalVariables|GetL_AbilityDefinitionFound)))))

(fn BPASCheckHasTags
  (params (ActorToCheck :type Actor%20Object%20Reference) (TagsToCheck :type Gameplay%20Tag%20Container%20Structure) (Has%20All? :type Boolean) (Has%20Any? :type Boolean) (Match%20All? :type Boolean))
  (Utilities|FlowControl|Sequence
    (:then_0
      (if Has%20All?
        (if (GameplayTags|HasAllTags (Variables|/Game/BPAS/Components/BPAS_GameplayTagManagerComponent.BPAS_GameplayTagManagerComponent_C|GetBPASGameplayTags (.BPAS%20Gameplay%20Tag%20Manager (CallFunction|BPASGetActorBPASSystem ActorToCheck ActorToCheck))) TagsToCheck Match%20All?)
          (return true))))
    (:then_1
      (if Has%20Any?
        (if (GameplayTags|HasAnyTags (Variables|/Game/BPAS/Components/BPAS_GameplayTagManagerComponent.BPAS_GameplayTagManagerComponent_C|GetBPASGameplayTags (.BPAS%20Gameplay%20Tag%20Manager (CallFunction|BPASGetActorBPASSystem ActorToCheck ActorToCheck))) TagsToCheck Match%20All?)
          (return true))))))

(fn BPASEditAttribute
  (params (BPAS%20Actor :type Actor%20Object%20Reference)))

(fn BPASCheckHasBPASSystem
  (params (ActorToCheck :type Actor%20Object%20Reference))
  (return (Utilities|IsValid (Actor|GetComponentbyClass ActorToCheck "/Game/BPAS/Components/BPAS_AbilityManagerComponent.BPAS_AbilityManagerComponent_C"))))

(fn BPASGetActorBPASSystem
  (params (BPAS%20Actor :type Actor%20Object%20Reference))
  ;[0.15 0.15 0.15 0.5] If actor has BPAS system, return all BPAS components
  (if (CallFunction|BPASCheckHasBPASSystem BPAS%20Actor BPAS%20Actor)
    (return (Actor|GetComponentbyClass BPAS%20Actor "/Game/BPAS/Components/BPAS_AbilityManagerComponent.BPAS_AbilityManagerComponent_C") (Actor|GetComponentbyClass BPAS%20Actor "/Game/BPAS/Components/BPAS_AttributeManagerComponent.BPAS_AttributeManagerComponent_C") (Actor|GetComponentbyClass BPAS%20Actor "/Game/BPAS/Components/BPAS_GameplayTagManagerComponent.BPAS_GameplayTagManagerComponent_C"))))

(fn BPASSendAbilityEvent
  (params (EventTag :type Gameplay%20Tag%20Structure) (EventContext :type Struct%20Ability%20Event%20Context%20Structure) (Actor :type Actor%20Object%20Reference))
  (bind _bpas_ability_manager (CallFunction|BPASGetActorBPASSystem Actor Actor))
  (Utilities|IsValid _bpas_ability_manager
    (:Is%20Valid
      (Default|BroadcastBPASEvent _bpas_ability_manager EventTag EventContext))))