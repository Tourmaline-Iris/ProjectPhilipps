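; Blueprint function library for adding, removing, finding and crafting items across a player's inventory and hotbar.
; Find functions gather matching or free slots and totals from both containers, optionally comparing item subdata.
; Add and Remove use those totals to refuse requests that cannot be met in full, with Add topping up partial stacks before filling empty slots.
; CraftItem checks every recipe requirement, consumes them, then adds the result.
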(fn RemoveItemfromInventory
  (params (Item :type Inventory%20Content%20Struct%20Structure) (PlayerRef :type First%20Person%20Character%20Object%20Reference) (MatchSubdata :type Boolean))
  (bind (_itemtype _quantity _subdata) (Utilities|Struct|BreakInventoryContentStruct Item))
  (bind (_quantityfound _slot_references) (CallFunction|FindItemonPlayer _itemtype _subdata PlayerRef MatchSubdata))
  (if (> _quantity _quantityfound)
    (return false)
    (else
      (LocalVariables|SetL_Item Item)
      (LocalVariables|SetL_QunatityToRemove _quantity)
      (bind _output_get (LocalVariables|SetL_SlotsToRemoveFrom _slot_references))
      (bind _array_element (Utilities|Array|ForEachLoopwithBreak _output_get :!label _label)
        (:LoopBody
          (if (== (LocalVariables|GetL_QunatityToRemove) 0)
            (goto _label Break)
            (elif (>= (.quantity (Default|GetItemInfoatIndex (Variables|/Game/InventorySystem/UI/WBP_InventorySlot.WBP_InventorySlot_C|GetInvRef _array_element) (Variables|/Game/InventorySystem/UI/WBP_InventorySlot.WBP_InventorySlot_C|GetIndex _array_element))) (LocalVariables|GetL_QunatityToRemove))
              (Default|RemovefromStack _array_element (LocalVariables|GetL_QunatityToRemove))
              (LocalVariables|SetL_QunatityToRemove 0)
              (else
                (Default|RemovefromStack _array_element (.quantity (Default|GetItemInfoatIndex (Variables|/Game/InventorySystem/UI/WBP_InventorySlot.WBP_InventorySlot_C|GetInvRef _array_element) (Variables|/Game/InventorySystem/UI/WBP_InventorySlot.WBP_InventorySlot_C|GetIndex _array_element))))
                (LocalVariables|SetL_QunatityToRemove (- (LocalVariables|GetL_QunatityToRemove) (.quantity (Default|GetItemInfoatIndex (Variables|/Game/InventorySystem/UI/WBP_InventorySlot.WBP_InventorySlot_C|GetInvRef _array_element) (Variables|/Game/InventorySystem/UI/WBP_InventorySlot.WBP_InventorySlot_C|GetIndex _array_element)))))))))
        (:Completed
          (return true))))))

(fn FindIteminInventory
  (params (Item :type BP%20Master%20Item%20Class%20Reference) (Subdata :type Item%20Subdata%20Struct%20Structure) (Inventory :type BP%20Inventory%20Component%20Object%20Reference) (MatchSubdata :type Boolean))
  (LocalVariables|SetL_MatchSubdata MatchSubdata)
  (LocalVariables|SetL_QuantityFound 0)
  (Utilities|Array|Clear (LocalVariables|GetL_StoredSlots))
  (LocalVariables|SetL_ItemToFind Item)
  (LocalVariables|SetL_Subdata Subdata)
  (LocalVariables|SetL_InvRef Inventory)
  (for (_array_element _array_index) (Variables|/Game/InventorySystem/BP_InventoryComponent.BP_InventoryComponent_C|GetContents Inventory)
    (if (and (== (.itemtype _array_element) (LocalVariables|GetL_ItemToFind)) (or (CallFunction|CompareSubdata (LocalVariables|GetL_Subdata) (.subdata _array_element)) (not (LocalVariables|GetL_MatchSubdata))))
      (LocalVariables|SetL_QuantityFound (+ (LocalVariables|GetL_QuantityFound) (.quantity _array_element)))
      (Utilities|Array|Add (LocalVariables|GetL_StoredSlots) (Utilities|Array|Get(acopy) (Variables|/Game/InventorySystem/BP_InventoryComponent.BP_InventoryComponent_C|GetSlotref (LocalVariables|GetL_InvRef)) _array_index))))
  (return (LocalVariables|GetL_QuantityFound) (LocalVariables|GetL_StoredSlots)))

(fn FindItemonPlayer
  (params (Item :type BP%20Master%20Item%20Class%20Reference) (Subdata :type Item%20Subdata%20Struct%20Structure) (PlayerRef :type First%20Person%20Character%20Object%20Reference) (MatchSubdata :type Boolean))
  (bind _l_slots (LocalVariables|GetL_Slots))
  (LocalVariables|SetL_MatchSubdata MatchSubdata)
  (Utilities|Array|Clear (LocalVariables|GetL_Slots))
  (LocalVariables|SetL_RunningTotal 0)
  (LocalVariables|SetL_ItemRef Item)
  (LocalVariables|SetL_Subdata Subdata)
  (bind _output_get (LocalVariables|SetL_PlayerRef PlayerRef))
  (Utilities|FlowControl|Sequence
    (:then_0
      (bind (_quantityfound _slotreferences) (CallFunction|FindIteminInventory (LocalVariables|GetL_ItemRef) (LocalVariables|GetL_Subdata) (Variables|/Game/FirstPersonBP/Blueprints/FirstPersonCharacter.FirstPersonCharacter_C|GetPlayerInventory _output_get) (LocalVariables|GetL_MatchSubdata)))
      (LocalVariables|SetL_RunningTotal (+ (LocalVariables|GetL_RunningTotal) _quantityfound))
      (for _array_element _slotreferences
        (Utilities|Array|Add _l_slots _array_element)))
    (:then_1
      (bind (_quantityfound_2 _slotreferences_2) (CallFunction|FindIteminInventory (LocalVariables|GetL_ItemRef) (LocalVariables|GetL_Subdata) (Variables|/Game/FirstPersonBP/Blueprints/FirstPersonCharacter.FirstPersonCharacter_C|GetPlayerHotbar _output_get) (LocalVariables|GetL_MatchSubdata)))
      (LocalVariables|SetL_RunningTotal (+ (LocalVariables|GetL_RunningTotal) _quantityfound_2))
      (for _array_element_2 _slotreferences_2
        (Utilities|Array|Add _l_slots _array_element_2)))
    (:then_2
      (return (LocalVariables|GetL_RunningTotal) (LocalVariables|GetL_Slots)))))

(fn AddItemtoInventory
  (params (PlayerRef :type First%20Person%20Character%20Object%20Reference) (ItemToAdd :type Inventory%20Content%20Struct%20Structure))
  (bind (_runningtotal _slots) (CallFunction|FindSpaceonPlayer PlayerRef (Utilities|Struct|MakeInventoryContentStruct (.itemtype ItemToAdd) (.quantity ItemToAdd) (.subdata ItemToAdd)) true))
  (if (> (.quantity ItemToAdd) _runningtotal)
    (return false)
    (else
      (LocalVariables|SetL_Item (.itemtype ItemToAdd))
      (LocalVariables|SetL_QuantityToAdd (.quantity ItemToAdd))
      (LocalVariables|SetL_Subdata (.subdata ItemToAdd))
      (bind _output_get (LocalVariables|SetL_Slots _slots))
      (Utilities|FlowControl|Sequence
        (:then_0
          (for _array_element _output_get
            (if (== (LocalVariables|GetL_QuantityToAdd) 0)
              (return true)
              (elif (Utilities|IsValidClass (.itemtype (Default|GetItemInfoatIndex (Variables|/Game/InventorySystem/UI/WBP_InventorySlot.WBP_InventorySlot_C|GetInvRef _array_element) (Variables|/Game/InventorySystem/UI/WBP_InventorySlot.WBP_InventorySlot_C|GetIndex _array_element))))
                (if (>= (+ (.quantity (Default|GetItemInfoatIndex (Variables|/Game/InventorySystem/UI/WBP_InventorySlot.WBP_InventorySlot_C|GetInvRef _array_element) (Variables|/Game/InventorySystem/UI/WBP_InventorySlot.WBP_InventorySlot_C|GetIndex _array_element))) (LocalVariables|GetL_QuantityToAdd)) (Variables|/Game/ItemSystem/ItemData/PDA_ItemData.PDA_ItemData_C|GetStackSize (.ItemData (Utilities|GetClassDefaults (LocalVariables|GetL_Item)))))
                  (LocalVariables|SetL_QuantityToAdd (- (LocalVariables|GetL_QuantityToAdd) (- (Variables|/Game/ItemSystem/ItemData/PDA_ItemData.PDA_ItemData_C|GetStackSize (.ItemData (Utilities|GetClassDefaults (.itemtype (Default|GetItemInfoatIndex (Variables|/Game/InventorySystem/UI/WBP_InventorySlot.WBP_InventorySlot_C|GetInvRef _array_element) (Variables|/Game/InventorySystem/UI/WBP_InventorySlot.WBP_InventorySlot_C|GetIndex _array_element)))))) (.quantity (Default|GetItemInfoatIndex (Variables|/Game/InventorySystem/UI/WBP_InventorySlot.WBP_InventorySlot_C|GetInvRef _array_element) (Variables|/Game/InventorySystem/UI/WBP_InventorySlot.WBP_InventorySlot_C|GetIndex _array_element))))))
                  (Default|AddtoStack _array_element (LocalVariables|GetL_Item) (- (Variables|/Game/ItemSystem/ItemData/PDA_ItemData.PDA_ItemData_C|GetStackSize (.ItemData (Utilities|GetClassDefaults (.itemtype (Default|GetItemInfoatIndex (Variables|/Game/InventorySystem/UI/WBP_InventorySlot.WBP_InventorySlot_C|GetInvRef _array_element) (Variables|/Game/InventorySystem/UI/WBP_InventorySlot.WBP_InventorySlot_C|GetIndex _array_element)))))) (.quantity (Default|GetItemInfoatIndex (Variables|/Game/InventorySystem/UI/WBP_InventorySlot.WBP_InventorySlot_C|GetInvRef _array_element) (Variables|/Game/InventorySystem/UI/WBP_InventorySlot.WBP_InventorySlot_C|GetIndex _array_element)))) (LocalVariables|GetL_Subdata))
                  (else
                    (Default|AddtoStack _array_element (LocalVariables|GetL_Item) (LocalVariables|GetL_QuantityToAdd) (LocalVariables|GetL_Subdata))
                    (LocalVariables|SetL_QuantityToAdd 0)))))))
        (:then_1
          (for _array_element_2 _output_get
            (if (== (LocalVariables|GetL_QuantityToAdd) 0)
              (return true)
              (elif (not (Utilities|IsValidClass (.itemtype (Default|GetItemInfoatIndex (Variables|/Game/InventorySystem/UI/WBP_InventorySlot.WBP_InventorySlot_C|GetInvRef _array_element_2) (Variables|/Game/InventorySystem/UI/WBP_InventorySlot.WBP_InventorySlot_C|GetIndex _array_element_2)))))
                (if (>= (LocalVariables|GetL_QuantityToAdd) (Variables|/Game/ItemSystem/ItemData/PDA_ItemData.PDA_ItemData_C|GetStackSize (.ItemData (Utilities|GetClassDefaults (LocalVariables|GetL_Item)))))
                  (LocalVariables|SetL_QuantityToAdd (- (LocalVariables|GetL_QuantityToAdd) (Variables|/Game/ItemSystem/ItemData/PDA_ItemData.PDA_ItemData_C|GetStackSize (.ItemData (Utilities|GetClassDefaults (LocalVariables|GetL_Item))))))
                  (Default|AddtoStack _array_element_2 (LocalVariables|GetL_Item) (Variables|/Game/ItemSystem/ItemData/PDA_ItemData.PDA_ItemData_C|GetStackSize (.ItemData (Utilities|GetClassDefaults (LocalVariables|GetL_Item)))) (LocalVariables|GetL_Subdata))
                  (else
                    (Default|AddtoStack _array_element_2 (LocalVariables|GetL_Item) (LocalVariables|GetL_QuantityToAdd) (LocalVariables|GetL_Subdata))
                    (LocalVariables|SetL_QuantityToAdd 0)))))))))))

(fn FindSpaceinInventory
  (params (Item :type Inventory%20Content%20Struct%20Structure) (Inventory :type BP%20Inventory%20Component%20Object%20Reference) (MatchSubdata :type Boolean))
  (LocalVariables|SetL_MatchSubdata MatchSubdata)
  (LocalVariables|SetL_FreeSpace 0)
  (Utilities|Array|Clear (LocalVariables|GetL_StoredSlots))
  (LocalVariables|SetL_Item Item)
  (bind _output_get (LocalVariables|SetL_InvRef Inventory))
  (for _array_element (Variables|/Game/InventorySystem/BP_InventoryComponent.BP_InventoryComponent_C|GetSlotref _output_get)
    (LocalVariables|SetL_TempSlot _array_element)
    (if (Utilities|IsValidClass (.itemtype (Default|GetItemInfoatIndex (Variables|/Game/InventorySystem/UI/WBP_InventorySlot.WBP_InventorySlot_C|GetInvRef (LocalVariables|GetL_TempSlot)) (Variables|/Game/InventorySystem/UI/WBP_InventorySlot.WBP_InventorySlot_C|GetIndex (LocalVariables|GetL_TempSlot)))))
      (if (Math|Boolean|ANDBoolean (!= (Variables|/Game/ItemSystem/ItemData/PDA_ItemData.PDA_ItemData_C|GetStackSize (.ItemData (Utilities|GetClassDefaults (.itemtype (LocalVariables|GetL_Item))))) (.quantity (Default|GetItemInfoatIndex (Variables|/Game/InventorySystem/UI/WBP_InventorySlot.WBP_InventorySlot_C|GetInvRef (LocalVariables|GetL_TempSlot)) (Variables|/Game/InventorySystem/UI/WBP_InventorySlot.WBP_InventorySlot_C|GetIndex (LocalVariables|GetL_TempSlot))))) (== (.itemtype (Default|GetItemInfoatIndex (Variables|/Game/InventorySystem/UI/WBP_InventorySlot.WBP_InventorySlot_C|GetInvRef (LocalVariables|GetL_TempSlot)) (Variables|/Game/InventorySystem/UI/WBP_InventorySlot.WBP_InventorySlot_C|GetIndex (LocalVariables|GetL_TempSlot)))) (.itemtype (LocalVariables|GetL_Item))) (or (CallFunction|CompareSubdata (.subdata (Default|GetItemInfoatIndex (Variables|/Game/InventorySystem/UI/WBP_InventorySlot.WBP_InventorySlot_C|GetInvRef (LocalVariables|GetL_TempSlot)) (Variables|/Game/InventorySystem/UI/WBP_InventorySlot.WBP_InventorySlot_C|GetIndex (LocalVariables|GetL_TempSlot)))) (.subdata (LocalVariables|GetL_Item))) (not (LocalVariables|GetL_MatchSubdata))))
        (Utilities|Array|Add (LocalVariables|GetL_StoredSlots) (LocalVariables|GetL_TempSlot))
        (LocalVariables|SetL_FreeSpace (+ (- (Variables|/Game/ItemSystem/ItemData/PDA_ItemData.PDA_ItemData_C|GetStackSize (.ItemData (Utilities|GetClassDefaults (.itemtype (LocalVariables|GetL_Item))))) (.quantity (Default|GetItemInfoatIndex (Variables|/Game/InventorySystem/UI/WBP_InventorySlot.WBP_InventorySlot_C|GetInvRef (LocalVariables|GetL_TempSlot)) (Variables|/Game/InventorySystem/UI/WBP_InventorySlot.WBP_InventorySlot_C|GetIndex (LocalVariables|GetL_TempSlot))))) (LocalVariables|GetL_FreeSpace))))
      (else
        (Utilities|Array|Add (LocalVariables|GetL_StoredSlots) (LocalVariables|GetL_TempSlot))
        (LocalVariables|SetL_FreeSpace (+ (LocalVariables|GetL_FreeSpace) (Variables|/Game/ItemSystem/ItemData/PDA_ItemData.PDA_ItemData_C|GetStackSize (.ItemData (Utilities|GetClassDefaults (.itemtype (LocalVariables|GetL_Item))))))))))
  (return (LocalVariables|GetL_StoredSlots) (LocalVariables|GetL_FreeSpace)))

(fn FindSpaceonPlayer
  (params (PlayerRef :type First%20Person%20Character%20Object%20Reference) (Item :type Inventory%20Content%20Struct%20Structure) (MatchSubdata :type Boolean))
  (bind _l_slots (LocalVariables|GetL_Slots))
  (LocalVariables|SetL_MatchSubdata MatchSubdata)
  (Utilities|Array|Clear (LocalVariables|GetL_Slots))
  (LocalVariables|SetL_RunningTotal 0)
  (LocalVariables|SetL_PlayerRef PlayerRef)
  (LocalVariables|SetL_ItemRef Item)
  (Utilities|FlowControl|Sequence
    (:then_0
      (bind (_validslots _freespace) (CallFunction|FindSpaceinInventory (LocalVariables|GetL_ItemRef) (Variables|/Game/FirstPersonBP/Blueprints/FirstPersonCharacter.FirstPersonCharacter_C|GetPlayerInventory (LocalVariables|GetL_PlayerRef)) (LocalVariables|GetL_MatchSubdata)))
      (LocalVariables|SetL_RunningTotal (+ (LocalVariables|GetL_RunningTotal) _freespace))
      (for _array_element _validslots
        (Utilities|Array|Add _l_slots _array_element)))
    (:then_1
      (bind (_validslots_2 _freespace_2) (CallFunction|FindSpaceinInventory (LocalVariables|GetL_ItemRef) (Variables|/Game/FirstPersonBP/Blueprints/FirstPersonCharacter.FirstPersonCharacter_C|GetPlayerHotbar (LocalVariables|GetL_PlayerRef)) (LocalVariables|GetL_MatchSubdata)))
      (LocalVariables|SetL_RunningTotal (+ (LocalVariables|GetL_RunningTotal) _freespace_2))
      (for _array_element_2 _validslots_2
        (Utilities|Array|Add _l_slots _array_element_2)))
    (:then_2
      (return (LocalVariables|GetL_RunningTotal) (LocalVariables|GetL_Slots)))))

(fn CraftItem
  (params (Recipe :type Crafting%20Recipe%20Struct%20Structure) (PlayerRef :type First%20Person%20Character%20Object%20Reference))
  (LocalVariables|SetL_Recipe Recipe)
  (LocalVariables|SetL_PlayerRef PlayerRef)
  (Utilities|FlowControl|Sequence
    (:then_0
      ;[1 1 1] Check all the recipe requirements are there
      (for _array_element (.Requirements (Utilities|Struct|BreakCraftingRecipeStruct (LocalVariables|GetL_Recipe)))
        (bind _quantityfound (CallFunction|FindItemonPlayer :Item (.itemtype _array_element) :PlayerRef (LocalVariables|GetL_PlayerRef)))
        (if (not (>= _quantityfound (.quantity _array_element)))
          (return false))))
    (:then_1
      ;[1 1 1] Consume cost items
      (for _array_element_2 (.Requirements (Utilities|Struct|BreakCraftingRecipeStruct (LocalVariables|GetL_Recipe)))
        (CallFunction|RemoveItemfromInventory (Utilities|Struct|MakeInventoryContentStruct (.itemtype _array_element_2) (.quantity _array_element_2) (.subdata _array_element_2)) (LocalVariables|GetL_PlayerRef) false)))
    (:then_2
      (CallFunction|AddItemtoInventory (LocalVariables|GetL_PlayerRef) (.ResultItem (Utilities|Struct|BreakCraftingRecipeStruct (LocalVariables|GetL_Recipe)))))))

(fn CompareSubdata
  (params (Item%201 :type Item%20Subdata%20Struct%20Structure) (Item%202 :type Item%20Subdata%20Struct%20Structure))
  (return (Utilities|Array|ContainsItem (Utilities|Array|MakeArray Item%201) Item%202)))